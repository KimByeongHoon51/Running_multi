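; Scene component that gives its owning character a name tag widget showing a name and HP, SP and FP values.
; On BeginPlay it creates the NameTag widget with a reference to itself, adds it to the viewport and initializes it with the attach parent's owning Character.
; Setter functions forward name and stat updates straight to the widget.
; EndPlay removes the widget from the viewport.
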(event `self.ReceiveBeginPlay`
  (bind _returnvalue (`|CreateWidget` "/Game/NameTag/NameTag.NameTag_C" null self))
  (bind _output_get (set `self.NameTag` _returnvalue))
  (`UserWidget.AddToViewport` _output_get 0)
  (bind _ascharacter (cast `Character` (`self.GetOwner` (`self.GetAttachParent`))))
  (`self.InitCharacter` _ascharacter))

(event `self.ReceiveEndPlay`
  (params (EndPlayReason :type "EEndPlayReason Enum" :default "Destroyed"))
  (`Widget.RemoveFromParent` (`self.NameTag`)))

(fn `InitCharacter`
  (params (Character :type "Character Object Reference"))
  (`/Game/NameTag/NameTag.InitCharacter` (`self.NameTag`) Character))

(fn `SetFP`
  (params (CurFP :type "Float (double-precision)") (MaxFP :type "Float (double-precision)"))
  (`/Game/NameTag/NameTag.SetFP` (`self.NameTag`) CurFP MaxFP))

(fn `SetHP`
  (params (CurHP :type "Float (double-precision)") (MaxHP :type "Float (double-precision)"))
  (`/Game/NameTag/NameTag.SetHp` (`self.NameTag`) CurHP MaxHP))

(fn `SetName`
  (params (Name :type String))
  (`/Game/NameTag/NameTag.SetName` (`self.NameTag`) Name))

(fn `SetSP`
  (params (CurSP :type "Float (double-precision)") (MaxSP :type "Float (double-precision)"))
  (`/Game/NameTag/NameTag.SetSP` (`self.NameTag`) CurSP MaxSP))