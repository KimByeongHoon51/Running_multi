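; Actor that spawns a random buff pickup from its BuffClass list at its own transform, named as the speed debuff spawner.
; It spawns on BeginPlay and binds to the spawned actor's OnDestroyed event.
; When that actor is destroyed, it waits RespawnDelay and spawns another random pick, keeping a continuous respawn cycle.
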(event `self.ReceiveBeginPlay`
  (`self.BuffSpawn`))

(event `BuffSpawn`
  (bind _returnvalue (`|SpawnActorFromClass` (`KismetArrayLibrary.Array_Random` (`self.BuffClass`)) (`self.GetTransform`) "Undefined" "MultiplyWithRoot" null null))
  (add `self.OnDestroyed` _returnvalue (`|CreateDelegate` :!event `OnBuffDestroyed`)))

(event `OnBuffDestroyed` :!signature `self.OnDestroyed`
  (params (DestroyedActor :type "Actor Object Reference"))
  (`KismetSystemLibrary.Delay` (`self.RespawnDelay`))
  (`self.BuffSpawn`))

(fn `UserConstructionScript`)