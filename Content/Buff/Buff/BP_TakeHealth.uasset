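; BP_TakeHealth is an overlap-triggered pickup actor that removes health from the player.
; On overlap with a BP_ThirdPersonCharacter, it attaches the BuffEffectToAttach Niagara effect to the character's mesh.
; It then subtracts a fixed amount directly from CurHP on the character's BP_PlayerState, with no clamping here, and destroys itself.
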(event `self.ReceiveActorBeginOverlap`
  (params (OtherActor :type "Actor Object Reference"))
  (bind _asbp_third_person_character (cast `/Game/ThirdPerson/Blueprints/BP_ThirdPersonCharacter` OtherActor))
  (bind _asbp_player_state (cast `/Game/GameMode/BP_PlayerState` (`Pawn.PlayerState` _asbp_third_person_character)))
  (`NiagaraFunctionLibrary.SpawnSystemAttached` (`self.BuffEffectToAttach`) (`Character.Mesh` _asbp_third_person_character) "None" (0.0 0.0 0.0) (struct) "SnapToTarget")
  (set `/Game/GameMode/BP_PlayerState.CurHP` (+ (`/Game/GameMode/BP_PlayerState.CurHP` _asbp_player_state) -30.0) _asbp_player_state)
  (`self.K2_DestroyActor`))

(fn `UserConstructionScript`
  (`parent.UserConstructionScript`))