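; Speed buff effect actor that raises the walk speed of the Character it is attached to while the effect exists.
; On BeginPlay it waits briefly, then casts its attach parent actor to Character and sets a higher MaxWalkSpeed.
; On EndPlay it casts the parent again and writes a fixed lower speed rather than restoring a saved original.
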(event `self.ReceiveBeginPlay`
  (`KismetSystemLibrary.Delay` 0.2)
  (bind _ascharacter (cast `Character` (`self.GetAttachParentActor`)))
  (set `CharacterMovementComponent.MaxWalkSpeed` 1000.0 (`Character.CharacterMovement` _ascharacter)))

(event `self.ReceiveEndPlay`
  (params (EndPlayReason :type "EEndPlayReason Enum" :default "Destroyed"))
  (bind _ascharacter (cast `Character` (`self.GetAttachParentActor`)))
  (set `CharacterMovementComponent.MaxWalkSpeed` 600.0 (`Character.CharacterMovement` _ascharacter)))

(fn `UserConstructionScript`
  (`parent.UserConstructionScript`))