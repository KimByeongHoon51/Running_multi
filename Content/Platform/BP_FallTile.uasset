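; BP_FallTile is a platform tile that drops away after something overlaps its Box trigger.
; The overlap runs ResFall, guarded by a short arming delay after BeginPlay and a flag against retriggering.
; A timeline tints the mesh's dynamic material from white to red as a warning.
; Delays chained off the timeline update then enable physics simulation and later destroy the actor.
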(event `self.ReceiveBeginPlay`
  (bind _staticmesh (`self.StaticMesh`))
  (set `self.bIsReadyToFall` false)
  (`KismetSystemLibrary.Delay` 0.2)
  (set `self.bIsReadyToFall` true)
  (`PrimitiveComponent.CreateDynamicMaterialInstance` _staticmesh 0 null "None")
  (`MeshComponent.SetVectorParameterValueOnMaterials` _staticmesh "Color" (1.0 1.0 1.0)))

(event `self.Box.OnComponentBeginOverlap`
  (params (OverlappedComponent :type "PrimitiveComponent Object Reference") (OtherActor :type "Actor Object Reference") (OtherComp :type "PrimitiveComponent Object Reference") (OtherBodyIndex :type Integer) (bFromSweep :type Boolean) (SweepResult :type "HitResult Structure (by ref)"))
  (`self.ResFall`))

(event `ResFall`
  (if (`self.bIsReadyToFall`)
    (if (not (`self.IsAlreadyFading`))
      (bind (_direction _time) (`Timeline|TL_ColorFade` :!via `PlayFromStart`)
        (:`Update`
          (set `self.IsAlreadyFading` true)
          (`MeshComponent.SetVectorParameterValueOnMaterials` (`self.StaticMesh`) "Color" (`KismetMathLibrary.Conv_LinearColorToVector` (`KismetMathLibrary.LinearColorLerp` (struct :`R` 1.0 :`G` 1.0 :`B` 1.0 :`A` 1.0) (struct :`R` 1.0 :`A` 1.0) _time)))
          (`KismetSystemLibrary.Delay` 0.8)
          (`PrimitiveComponent.SetSimulatePhysics` (`self.StaticMesh`) true)
          (`KismetSystemLibrary.Delay` 2.0)
          (`self.K2_DestroyActor`))))))

(fn `UserConstructionScript`)