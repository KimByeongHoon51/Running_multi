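; Lobby HUD Blueprint that shows the lobby widget and keeps its player list in sync with player states.
; BeginPlay creates the widget, switches to UI-only input and shows the mouse cursor.
; BindPlayerState hooks a player state's nickname-change and destroyed events, which refresh the player list.
; The refresh retries on a short timer until the widget is valid, covering binds that arrive before it is created.
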(event `self.ReceiveBeginPlay`
  (bind _returnvalue (`GameplayStatics.GetPlayerController` 0))
  (bind _returnvalue_2 (`|CreateWidget` "/Game/Blueprints/Widgets/Lobby/LobbyHUDWidget.LobbyHUDWidget_C"))
  (bind _output_get (set `self.LobbyHUDWidget` _returnvalue_2))
  (`UserWidget.AddToViewport` _output_get 0)
  (`WidgetBlueprintLibrary.SetInputMode_UIOnlyEx` _returnvalue null)
  (set `PlayerController.bShowMouseCursor` true _returnvalue))

(fn `BindPlayerState`
  (params (PlayerState :type "/Game/Blueprints/Game/Lobby/BP_LobbyPlayerState Object Reference"))
  (add `/Game/Blueprints/Game/Lobby/BP_LobbyPlayerState.EventDispatcher_ChangeNickName` PlayerState (`|CreateDelegate` :!event `EventChangeNickName`))
  (`self.EventChangeNickName` (`/Game/Blueprints/Game/Lobby/BP_LobbyPlayerState.NickName` PlayerState))
  (add `self.OnDestroyed` PlayerState (`|CreateDelegate` :!event `DestroyNickName`)))

(fn `DestroyNickName`
  (params (DestroyedActor :type "Actor Object Reference"))
  (`self.UpdateChangeNickName`))

(fn `EventChangeNickName`
  (params (NickName :type String))
  (`self.UpdateChangeNickName`))

(fn `UpdateChangeNickName`
  (bind _lobbyhudwidget (`self.LobbyHUDWidget`)
    (:`then`
      (`/Game/Blueprints/Widgets/Lobby/LobbyHUDWidget.UpdatePlayerList` _lobbyhudwidget))
    (:`else`
      (`KismetSystemLibrary.K2_SetTimer` null "UpdateChangeNickName" 0.01))))

(fn `UserConstructionScript`)