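; BP_BasicPillar is a pillar obstacle that damages and launches characters overlapping its cylinder.
; DoDamage finds each overlapping BP_ThirdPersonCharacter and applies Damage, crediting player controller 0 as instigator.
; It then launches the character along its own forward vector scaled by KnockBack, overriding velocity, and attaches a buff effect system to its mesh.
; Nothing in this file calls DoDamage, and the construction script is empty.
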(fn `DoDamage`
  (for _array_element (`PrimitiveComponent.GetOverlappingActors` (`self.Cylinder`) "/Game/ThirdPerson/Blueprints/BP_ThirdPersonCharacter.BP_ThirdPersonCharacter_C")
    (`GameplayStatics.ApplyDamage` _array_element (`self.Damage`) (`GameplayStatics.GetPlayerController` 0) self)
    (bind _ascharacter (cast `Character` _array_element))
    (`Character.LaunchCharacter` _ascharacter (* (`self.GetActorForwardVector` _ascharacter) (`self.KnockBack`)) true true)
    (`NiagaraFunctionLibrary.SpawnSystemAttached` (`self.BuffEffectToAttach`) (`Character.Mesh` _ascharacter) "None" (0.0 0.0 100.0) (struct) "SnapToTarget")))

(fn `UserConstructionScript`)