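; Gravity-flip obstacle that inverts the third-person character's gravity when it touches the cube.
; On overlap it makes the character jump, then toggles gravity scale between normal and negative based on its current sign.
; It also updates the character's reverse-gravity flag and moves and rotates the mesh so the character appears upside down or upright to match.
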(event `self.Cube.OnComponentBeginOverlap`
  (params (OverlappedComponent :type "PrimitiveComponent Object Reference") (OtherActor :type "Actor Object Reference") (OtherComp :type "PrimitiveComponent Object Reference") (OtherBodyIndex :type Integer) (bFromSweep :type Boolean) (SweepResult :type "HitResult Structure (by ref)"))
  (bind _asbp_third_person_character (cast `/Game/ThirdPerson/Blueprints/BP_ThirdPersonCharacter` OtherActor))
  (`Character.Jump` _asbp_third_person_character)
  (bind _charactermovement (`Character.CharacterMovement` _asbp_third_person_character))
  (if (< (`CharacterMovementComponent.GravityScale` _charactermovement) 0.0)
    (set `/Game/ThirdPerson/Blueprints/BP_ThirdPersonCharacter.bIsGravityReverse` false _asbp_third_person_character)
    (set `CharacterMovementComponent.GravityScale` 1.75 _charactermovement)
    (bind _mesh (`Character.Mesh` _asbp_third_person_character))
    (`SceneComponent.K2_SetRelativeLocationAndRotation` _mesh (0.0 0.0 -100.0) (struct :`Yaw` -90.0) false false)
    (else
      (set `/Game/ThirdPerson/Blueprints/BP_ThirdPersonCharacter.bIsGravityReverse` true _asbp_third_person_character)
      (set `CharacterMovementComponent.GravityScale` -1.75 _charactermovement)
      (`SceneComponent.K2_SetRelativeLocationAndRotation` _mesh (0.0 0.0 100.0) (struct :`Pitch` 180.0 :`Yaw` -90.0) false false))))

(fn `UserConstructionScript`)