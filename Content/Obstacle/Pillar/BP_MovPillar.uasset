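; BP_MovPillar is an obstacle pillar that shuttles between its starting position and a point MoveDistance away along world Y.
; On BeginPlay, only the authority calls ReqMove, which stores both endpoints and plays a timeline.
; The timeline lerps the actor's location without sweeping, and on finishing flips MoveRight to choose between Reverse and Play, repeating the motion.
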(event `self.ReceiveBeginPlay`
  (`/Engine/EditorBlueprintResources/ActorMacros.Switch Has Authority`
    (:`Authority`
      (`self.ReqMove`))))

(event `ReqMove`
  (bind _output_get (set `self.StartLocation` (`self.K2_GetActorLocation`)))
  (set `self.EndLocation` (+ _output_get (`KismetMathLibrary.MakeVector` 0.0 (`self.MoveDistance`))))
  (bind (_direction _newtrack_0) (`Timeline|Timeline` :!label _label)
    (:`Update`
      (`self.K2_SetActorLocation` (`KismetMathLibrary.VLerp` (`self.StartLocation`) (`self.EndLocation`) _newtrack_0)))
    (:`Finished`
      (if (`self.bMoveRight`)
        (set `self.bMoveRight` false)
        (goto _label :!via `Reverse`)
        (else
          (set `self.bMoveRight` true)
          (goto _label))))))

(fn `UserConstructionScript`
  (`parent.UserConstructionScript`))