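; BP_ObstacleBase is a base obstacle that damages and knocks back the third-person character on contact.
; A capsule begin-overlap calls DoDamage when CanDamage is set, then blocks further hits for DamageCoolTime.
; DoDamage applies Damage to each overlapping BP_ThirdPersonCharacter, crediting player controller 0.
; It launches each along the character's own forward vector scaled by KnockBack, overriding existing velocity.
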(event `self.Capsule.OnComponentBeginOverlap`
  (params (OverlappedComponent :type "PrimitiveComponent Object Reference") (OtherActor :type "Actor Object Reference") (OtherComp :type "PrimitiveComponent Object Reference") (OtherBodyIndex :type Integer) (bFromSweep :type Boolean) (SweepResult :type "HitResult Structure (by ref)"))
  (if (`self.bCanDamage`)
    (`self.DoDamage`)
    (set `self.bCanDamage` false)
    (`KismetSystemLibrary.Delay` (`self.DamageCoolTime`))
    (set `self.bCanDamage` true)))

(event `self.ReceiveBeginPlay`)

(fn `DoDamage`
  (for _array_element (`PrimitiveComponent.GetOverlappingActors` (`self.Capsule`) "/Game/ThirdPerson/Blueprints/BP_ThirdPersonCharacter.BP_ThirdPersonCharacter_C")
    (`GameplayStatics.ApplyDamage` _array_element (`self.Damage`) (`GameplayStatics.GetPlayerController` 0) self)
    (bind _ascharacter (cast `Character` _array_element))
    (`Character.LaunchCharacter` _ascharacter (* (`self.GetActorForwardVector` _ascharacter) (`self.KnockBack`)) true true)))

(fn `UserConstructionScript`)