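; BP_Spin is a spinning obstacle that damages and launches player characters on contact.
; Tick continuously yaws the scene component at RotationSpeed.
; An overlap on any of three boxes damages every BP_ThirdPersonCharacter inside them, then pauses further damage for DamageCoolTime.
; Knockback launches each character along its own forward vector scaled by KnockBack, and a character overlapping several boxes is hit once per box.
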(event `self.Box1.OnComponentBeginOverlap`
  (params (OverlappedComponent :type "PrimitiveComponent Object Reference") (OtherActor :type "Actor Object Reference") (OtherComp :type "PrimitiveComponent Object Reference") (OtherBodyIndex :type Integer) (bFromSweep :type Boolean) (SweepResult :type "HitResult Structure (by ref)"))
  (`self.HandleOverlap` :!label _label))

(event `HandleOverlap`
  (if (`self.bCanDamage`)
    (`self.DoDamage`)
    (set `self.bCanDamage` false)
    (`KismetSystemLibrary.Delay` (`self.DamageCoolTime`))
    (set `self.bCanDamage` true)))

(event `self.Box2.OnComponentBeginOverlap`
  (params (OverlappedComponent :type "PrimitiveComponent Object Reference") (OtherActor :type "Actor Object Reference") (OtherComp :type "PrimitiveComponent Object Reference") (OtherBodyIndex :type Integer) (bFromSweep :type Boolean) (SweepResult :type "HitResult Structure (by ref)"))
  (goto _label))

(event `self.ReceiveTick`
  (params (DeltaSeconds :type "Float (single-precision)"))
  (`SceneComponent.K2_AddLocalRotation` (`self.Scene`) (`KismetMathLibrary.MakeRotator` 0.0 0.0 (* DeltaSeconds (`self.RotationSpeed`))) false false))

(event `self.Box.OnComponentBeginOverlap`
  (params (OverlappedComponent :type "PrimitiveComponent Object Reference") (OtherActor :type "Actor Object Reference") (OtherComp :type "PrimitiveComponent Object Reference") (OtherBodyIndex :type Integer) (bFromSweep :type Boolean) (SweepResult :type "HitResult Structure (by ref)"))
  (goto _label))

(event `self.ReceiveBeginPlay`
  (set `self.CollisionArray` (`|MakeArray` (`self.Box1`) (`self.Box2`) (`self.Box`))))

(fn `DoDamage`
  (for _array_element (`self.CollisionArray`)
    (for _array_element_2 (`PrimitiveComponent.GetOverlappingActors` _array_element "/Game/ThirdPerson/Blueprints/BP_ThirdPersonCharacter.BP_ThirdPersonCharacter_C")
      (`GameplayStatics.ApplyDamage` _array_element_2 (`self.Damage`) (`GameplayStatics.GetPlayerController` 0) self)
      (bind _ascharacter (cast `Character` _array_element_2))
      (`Character.LaunchCharacter` _ascharacter (* (`self.GetActorForwardVector` _ascharacter) (`self.KnockBack`)) true true))))

(fn `UserConstructionScript`)