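; BP_BrainFullActivate is a two-choice quiz obstacle that pairs a question with left and right fake walls.
; On BeginPlay the authority picks a random question from the QuizCategory pool into the replicated Question variable.
; Its OnRep caches the BP_FakeWall child actors, sets the question and answer texts, then flags the wall matching the correct answer index with IsAnswer.
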(event `self.ReceiveBeginPlay`
  (`/Engine/EditorBlueprintResources/ActorMacros.Switch Has Authority`
    (:`Authority`
      (bind _randomquiz (`self.PickRandomQuestion`))
      (set `self.Question` _randomquiz))))

(fn `IsCorrect`
  (params (QuestionData :type "/Game/Obstacle/BrainFullActivate/Quiz/DA_Question Object Reference"))
  (if (== (`/Game/Obstacle/BrainFullActivate/Quiz/DA_Question.CorrectAnswer` QuestionData) 0)
    (set `/Game/Obstacle/BrainFullActivate/BP_FakeWall.bIsAnswer` true (`self.FakeWallL`))
    (else
      (set `/Game/Obstacle/BrainFullActivate/BP_FakeWall.bIsAnswer` true (`self.FakeWallR`)))))

(fn `OnRep_Question`
  (bind _question (`self.Question`))
  (bind _multiplechoice (`/Game/Obstacle/BrainFullActivate/Quiz/DA_Question.MultipleChoice` _question))
  (`|ExecutionSequence`
    (:`then_0`
      (bind _asbp_fake_wall (cast `/Game/Obstacle/BrainFullActivate/BP_FakeWall` (`ChildActorComponent.ChildActor` (`self.FakeWall_L`))))
      (set `self.FakeWallL` _asbp_fake_wall)
      (bind _asbp_fake_wall_2 (cast `/Game/Obstacle/BrainFullActivate/BP_FakeWall` (`ChildActorComponent.ChildActor` (`self.FakeWall_R`))))
      (set `self.FakeWallR` _asbp_fake_wall_2))
    (:`then_1`
      (`TextRenderComponent.K2_SetText` (`self.QuestionText`) (`/Game/Obstacle/BrainFullActivate/Quiz/DA_Question.Question` _question))
      (`TextRenderComponent.K2_SetText` (`self.LeftAnswerText`) (`|GetArrayItem` _multiplechoice))
      (`TextRenderComponent.K2_SetText` (`self.RightAnswerText`) (`|GetArrayItem` _multiplechoice 1))
      (`self.IsCorrect` _question))))

(fn `PickRandomQuestion`
  (returns (RandomQuiz :type "/Game/Obstacle/BrainFullActivate/Quiz/DA_Question Object Reference"))
  (bind _questionpool (`/Game/Obstacle/BrainFullActivate/Quiz/DA_Category.QuestionPool` (`self.QuizCategory`)))
  (return (`|GetArrayItem` _questionpool (`KismetMathLibrary.RandomIntegerInRange` 0 (- (`KismetArrayLibrary.Array_Length` _questionpool) 1)))))

(fn `UserConstructionScript`)