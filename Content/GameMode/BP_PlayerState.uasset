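; Player State that tracks stamina (SP), an HP gauge that fills with damage, and a fever gauge (FP).
; Tick drains SP while running, stopping the run when empty, and otherwise regenerates it without a cap.
; Full HP triggers fever, draining FP until empty, then HP resets to zero and FP refills.
; OnRep functions broadcast gauge changes through event dispatchers, and AddDamage also broadcasts HP directly.
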(event `self.ReceiveBeginPlay`
  (set `self.CurSP` (`self.MaxSP`))
  (set `self.CurFP` (`self.MaxFP`)))

(event `self.ReceiveTick`
  (params (DeltaSeconds :type "Float (single-precision)"))
  (`|ExecutionSequence`
    (:`then_0`
      (if (`self.IsRunning`)
        (`self.UseSP` (* DeltaSeconds 50.0))
        (if (not (`self.IsCanRun`))
          (set `self.IsRunning` false))
        (else
          (`self.RecvSP` (* DeltaSeconds 10.0)))))
    (:`then_1`
      (if (>= (`self.CurHP`) (`self.MaxHP`))
        (set `self.bIsFever` true)
        (`self.UseFP` (* DeltaSeconds 15.0))
        (if (<= (`self.CurFP`) 0.0)
          (set `self.CurHP` 0.0)
          (set `self.CurFP` (`self.MaxFP`)))
        (else
          (set `self.bIsFever` false))))))

(fn `AddDamage`
  (params (Damage :type "Float (double-precision)"))
  (bind _output_get (set `self.CurHP` (+ (`self.CurHP`) Damage)))
  (`self.EventDispatcher_UpdateHP` _output_get (`self.MaxHP`)))

(fn `DoRun`
  (params (IsRunning :type Boolean))
  (if IsRunning
    (set `self.IsRunning` true)
    (else
      (set `self.IsRunning` false))))

(fn `IsCanRun`
  (returns (IsCanRun :type Boolean))
  (return (> (`self.CurSP`) 0.0)))

(fn `OnRep_CurFP`
  (`self.EventDispatcher_UpdateFP` (`self.CurFP`) (`self.MaxFP`)))

(fn `OnRep_CurHP`
  (`self.EventDispatcher_UpdateHP` (`self.CurHP`) (`self.MaxHP`)))

(fn `OnRep_CurSP`
  (`self.EventDispatcher_UpdateSP` (`self.CurSP`) (`self.MaxSP`)))

(fn `RecvSP`
  (params (RecvSP :type "Float (double-precision)"))
  (set `self.CurSP` (+ (`self.CurSP`) RecvSP)))

(fn `UseFP`
  (params (UseFP :type "Float (double-precision)"))
  (set `self.CurFP` (`KismetMathLibrary.FClamp` (- (`self.CurFP`) UseFP) 0.0 (`self.MaxFP`))))

(fn `UserConstructionScript`)

(fn `UseSP`
  (params (UseSP :type "Float (double-precision)"))
  (set `self.CurSP` (`KismetMathLibrary.FClamp` (- (`self.CurSP`) UseSP) 0.0 (`self.MaxSP`))))